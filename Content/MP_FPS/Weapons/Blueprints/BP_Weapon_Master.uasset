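; Master weapon Blueprint for a multiplayer FPS, handling hitscan firing, damage and effects.
; On client fire, a camera sphere trace finds the aim point and a second traces toward it from the first-person muzzle.
; The server applies damage from that client-supplied hit without validation, then multicasts sound and effects.
; Muzzle flashes are split between owner-only first-person and owner-hidden third-person meshes; stop-fire is an empty stub.
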(event Custom|Client_OnWeaponFire
  (bind _bpcharactermasterref (Variables|Default|GetBPCharacterMasterRef))
  (bind _array (Utilities|Array|MakeArray _bpcharactermasterref))
  (bind _fp_cam (Variables|/Game/MP_FPS/Characters/Blueprints/BP_Character_Master.BP_Character_Master_C|GetFP_Cam _bpcharactermasterref))
  (bind _returnvalue (Transformation|GetWorldLocation _fp_cam))
  (bind (_outhit _returnvalue_2) (Collision|SphereTraceByChannel _returnvalue (+ _returnvalue (* (Math|Vector|GetForwardVector (Transformation|GetWorldRotation _fp_cam)) (Variables|Default|GetSphereTtraceRange))) (Variables|Default|GetSphereTraceRadius) "TraceTypeQuery1" false _array "None"))
  (bind (_outhit_2 _returnvalue_3) (Collision|SphereTraceByChannel (Transformation|GetSocketLocation (Variables|Default|GetSK_FP_Mesh_Weapon) (Variables|Default|GetMuzzleSocketNmae)) (Math|Vector|SelectVector (.ImpactPoint (Collision|BreakHitResult _outhit)) (.TraceEnd (Collision|BreakHitResult _outhit)) _returnvalue_2) (Variables|Default|GetSphereTraceRadius) "TraceTypeQuery1" false _array "None"))
  (CallFunction|ServerShootInfo _outhit_2 _returnvalue_3))

(event Custom|Server_ShootInfo
  (params (HitResult :type Hit%20Result%20Structure) (Hit :type Boolean))
  (Game|Damage|ApplyDamage (.HitActor (Collision|BreakHitResult HitResult)) (Math|Conversions|ToFloat(Integer) (Variables|Default|GetDamage)) (Game|GetInstigatorController) self)
  (CallFunction|Multicast-WeaponFX HitResult Hit))

(event Custom|Client_OffWeaponFire)

(event Custom|Multicast-WeaponFX
  (params (HitResult :type Hit%20Result%20Structure) (Hit :type Boolean))
  (bind (_bblockinghit _binitialoverlap _time _location _impactpoint _normal _impactnormal) (Collision|BreakHitResult HitResult))
  (bind _sk_fp_mesh_weapon (Variables|Default|GetSK_FP_Mesh_Weapon))
  (bind _muzzlesocketnmae (Variables|Default|GetMuzzleSocketNmae))
  (bind _psmuzzleflash (Variables|Default|GetPSMuzzleFlash))
  (Audio|SpawnSoundAttached (Variables|Default|GetFireWeaponSound) _sk_fp_mesh_weapon "MuzzleFlash")
  (Utilities|FlowControl|Sequence
    (:then_0
      (bind _returnvalue (Effects|SpawnEmitterAttached _psmuzzleflash _sk_fp_mesh_weapon _muzzlesocketnmae "0.000000, 0, 0" "0, 0, 0" "SnapToTarget"))
      (Rendering|SetOnlyOwnerSee _returnvalue true :!class /Script/Engine.PrimitiveComponent)
      (if Hit
        (Audio|PlaySoundatLocation (Variables|Default|GetImpactSound) _impactpoint)
        (Effects|SpawnEmitteratLocation (Variables|Default|GetPSImpact) "0, 0, 0" (Math|Rotator|MakeRotfromZ _impactnormal))))
    (:then_1
      (bind _returnvalue_2 (Effects|SpawnEmitterAttached _psmuzzleflash (Variables|Default|GetSK_TP_Weapon) _muzzlesocketnmae "0, 0, 0" "0, 0, 0" "SnapToTarget"))
      (Class|PrimitiveComponent|SetOwnerNoSee _returnvalue_2 true))))

(fn ConstructionScript)